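; Player pawn for the coin game, with a health bar HUD and a visual mesh that rolls as it moves.
; Each tick spins the mesh root from the last movement input and collision sphere circumference, an approximation that ignores actual velocity.
; Tick also watches health on MainPawnState_BP and triggers death once.
; Death shows the Game Over screen, spawns an explosion, destroys the mesh, disables input, and hides the health bar and game mode's start countdown.
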(event `self.ReceiveBeginPlay`
  ;[1 1 1] Create Health Bar HUD
  (bind _returnvalue (`|CreateWidget` "/Game/UI/HealthBarHUD.HealthBarHUD_C"))
  (bind _output_get (set `self.HealthBarReference` _returnvalue))
  (`UserWidget.AddToViewport` _output_get 0)
  (`Widget.SetVisibility` _output_get "Visible")
  (`WidgetBlueprintLibrary.SetInputMode_GameOnly` (`GameplayStatics.GetPlayerController` 0)))

(event `self.ReceiveTick`
  (params (DeltaSeconds :type "Float (single-precision)"))
  (`self.VisualMovementRotation` DeltaSeconds)
  ;[1 1 1] Death Detection/Event Call
  (bind _asmain_pawn_state_bp (cast `/Game/MainPawnState_BP` (`self.PlayerState`)))
  (if (`MainPawnState.Dead` _asmain_pawn_state_bp)
    _
    (elif (<= (`MainPawnState.CurrentHealth` _asmain_pawn_state_bp) 0.0)
      (`self.PlayerDied`)
      (set `MainPawnState.Dead` true _asmain_pawn_state_bp))))

(event `PlayerDied`
  (bind _returnvalue (`GameplayStatics.GetPlayerController` 0))
  ;[1 1 1] Show Death Screen
  (bind _returnvalue_2 (`|CreateWidget` "/Game/UI/GameOver.GameOver_C"))
  (`UserWidget.AddToViewport` _returnvalue_2 0)
  (`WidgetBlueprintLibrary.SetInputMode_UIOnlyEx` _returnvalue _returnvalue_2)
  (set `PlayerController.bShowMouseCursor` true _returnvalue)
  ;[1 1 1] Particle upon death
  (`GameplayStatics.SpawnEmitterAtLocation` (`self.ParticleExplosionReference`) (`self.K2_GetActorLocation`) (struct) (3.0 3.0 3.0))
  (`ActorComponent.K2_DestroyComponent` (`self.VisualMesh`))
  (`self.DisableInput` (`GameplayStatics.GetPlayerController` 0))
  (`Widget.SetVisibility` (`self.HealthBarReference`) "Hidden")
  ;[1 1 1] Hide countdown after (early) death
  (bind _ascoin_game_game_mode_base_bp (cast `/Game/CoinGameGameModeBase_BP` (`GameplayStatics.GetGameMode`)))
  (`Widget.SetVisibility` (`/Game/CoinGameGameModeBase_BP.GameStartCountdownReference` _ascoin_game_game_mode_base_bp) "Hidden"))

(fn `UserConstructionScript`)

(fn `VisualMovementRotation`
  (params (DeltaTime :type "Float (double-precision)"))
  (`SceneComponent.K2_AddWorldRotation` (`self.VisualMeshRoot`) (`KismetMathLibrary.MakeRotator` (.y (* (* (`KismetMathLibrary.Normal` (`self.GetLastMovementInputVector`)) DeltaTime) (`KismetMathLibrary.MultiplyByPi` (* 2 (`SphereComponent.GetScaledSphereRadius` (`self.CollisionMesh`)))))) (* -1 (.x (* (* (`KismetMathLibrary.Normal` (`self.GetLastMovementInputVector`)) DeltaTime) (`KismetMathLibrary.MultiplyByPi` (* 2 (`SphereComponent.GetScaledSphereRadius` (`self.CollisionMesh`)))))))) false false))