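; Game mode Blueprint for the coin game that runs a timed countdown before play starts.
; BeginPlay adds a countdown widget, and Tick updates it with the whole seconds left until StartDuration has passed since the game mode's creation.
; It then sets GameStarted on the game state and fires the GameStarted event, which removes the countdown and reveals player 0's score text above the health bar.
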(event `self.ReceiveBeginPlay`
  (bind _returnvalue (`|CreateWidget` "/Game/UI/GameStartCountdown.GameStartCountdown_C"))
  (bind _output_get (set `self.GameStartCountdownReference` _returnvalue))
  (`UserWidget.AddToViewport` _output_get 0))

(event `self.ReceiveTick`
  (params (DeltaSeconds :type "Float (single-precision)"))
  (bind _returnvalue (`self.GetGameTimeSinceCreation`))
  (bind _startduration (`self.StartDuration`))
  (bind _ascoin_game_game_state_base_bp (cast `/Game/CoinGameGameStateBase_BP` (`GameplayStatics.GetGameState`)))
  (if (`CoinGameGameStateBase.GameStarted` _ascoin_game_game_state_base_bp)
    _
    (elif (> _returnvalue _startduration)
      (set `CoinGameGameStateBase.GameStarted` true _ascoin_game_game_state_base_bp)
      (`self.GameStarted`)
      (else
        (`/Game/UI/GameStartCountdown.SetCountdown` (`self.GameStartCountdownReference`) (+ (`KismetMathLibrary.FTrunc` (- _startduration _returnvalue)) 1))))))

(event `GameStarted`
  (`Widget.RemoveFromParent` (`self.GameStartCountdownReference`))
  ;[1 1 1] Only show score above health bar after game starts
  (bind _asmain_pawn_bp (cast `/Game/MainPawn_BP` (`GameplayStatics.GetPlayerPawn` 0)))
  (`Widget.SetVisibility` (`/Game/UI/HealthBarHUD.ScoreText` (`/Game/MainPawn_BP.HealthBarReference` _asmain_pawn_bp)) "Visible"))

(fn `UserConstructionScript`)